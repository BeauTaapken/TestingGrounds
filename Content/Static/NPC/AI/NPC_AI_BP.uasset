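; NPC AI controller that runs a guard behavior tree and tracks sensed actors as targets.
; On BeginPlay it sets up the PatrolData blackboard and starts the GuardBehaviour tree.
; Perception updates write any actor lacking the "Enemy" tag to the enemy blackboard key when sensed.
; A failed sense of such an actor clears that key, without checking which actor it holds.
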(event `self.ReceiveBeginPlay`
  (bind _blackboardcomponent (`self.UseBlackboard` "/Game/Static/NPC/AI/PatrolData.PatrolData"))
  (`self.RunBehaviorTree` "/Game/Static/NPC/AI/GuardBehaviour.GuardBehaviour")
  (set `self.Blackboard Component` _blackboardcomponent))

(event `self.AIPerception.OnTargetPerceptionUpdated`
  (params (Actor :type "Actor Object Reference") (Stimulus :type "AIStimulus Structure"))
  (bind _blackboard_component (`self.Blackboard Component`))
  (bind _enemykey (`self.EnemyKey`))
  (if (`self.ActorHasTag` Actor "Enemy")
    _
    (elif (`.bSuccessfullySensed` (break `AIStimulus` Stimulus))
      (`BlackboardComponent.SetValueAsObject` _blackboard_component _enemykey Actor)
      (else
        (`BlackboardComponent.ClearValue` _blackboard_component _enemykey)))))

(fn `UserConstructionScript`)